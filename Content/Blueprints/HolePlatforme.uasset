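; HolePlatforme is a clickable platform Blueprint, likely a puzzle element, that switches on visually when first clicked.
; While it is inactive, a click fires a click dispatcher for listeners.
; A DoOnce then swaps the material on its four mesh components to a glowing "button on" material and sets Active, so further clicks are ignored.
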(fn `onClick`
  (if (not (`self.Active`))
    (`self.ClickDispatcher`)
    (`/Engine/EditorBlueprintResources/StandardMacros.DoOnce` false
      (:`Completed`
        (`PrimitiveComponent.SetMaterial` (`self.StaticMesh2`) 0 "/Game/Materials/GlowEnhanced_ButOn.GlowEnhanced_ButOn")
        (`PrimitiveComponent.SetMaterial` (`self.StaticMesh1`) 0 "/Game/Materials/GlowEnhanced_ButOn.GlowEnhanced_ButOn")
        (`PrimitiveComponent.SetMaterial` (`self.Cube 1`) 0 "/Game/Materials/GlowEnhanced_ButOn.GlowEnhanced_ButOn")
        (`PrimitiveComponent.SetMaterial` (`self.Cube`) 0 "/Game/Materials/GlowEnhanced_ButOn.GlowEnhanced_ButOn")
        (set `self.Active` true)))))

(fn `UserConstructionScript`)